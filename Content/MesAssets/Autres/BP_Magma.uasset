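; BP_Magma is a lava hazard that kills the BP_LavaMan player on contact unless the character has fire resistance.
; It caches the player character on BeginPlay, and a box collider overlap calls ColLavaPerso, which passes negated current health to GestionVie on that cached reference.
; An unconnected node chain holds an alternative response: fixed damage with a boosted jump, then a jump height reset.
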(event `self.ReceiveBeginPlay`
  (bind _asbp_lava_man (cast `/Game/MesAssets/BP_LavaMan` (`GameplayStatics.GetPlayerCharacter` 0)))
  (set `self.persoRef` _asbp_lava_man))

(event `self.BoxCollider.OnComponentBeginOverlap`
  (params (OverlappedComponent :type "PrimitiveComponent Object Reference") (OtherActor :type "Actor Object Reference") (OtherComp :type "PrimitiveComponent Object Reference") (OtherBodyIndex :type Integer) (bFromSweep :type Boolean) (SweepResult :type "HitResult Structure (by ref)"))
  ;[1 0.3438 0.6684] Collision personnage avec lave
  (cast `/Game/MesAssets/BP_LavaMan` OtherActor)
  (`self.ColLavaPerso`))

(fn `ColLavaPerso`
  (bind _persoref (`self.persoRef`))
  (if (not (`/Game/MesAssets/BP_LavaMan.fireResistance` _persoref))
    (`/Game/MesAssets/BP_LavaMan.gestionVie` _persoref (* (`/Game/MesAssets/BP_LavaMan.vie` _persoref) -1))))

(fn `UserConstructionScript`)