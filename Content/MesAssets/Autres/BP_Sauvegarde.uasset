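; BP_Sauvegarde is a save-game Blueprint for a coin or piece count (NbPieces), with a Sauvegarder function meant to save it.
; Sauvegarder checks whether the SaveName slot exists, then loads that save or creates a new BP_Sauvegarde object.
; It then assigns NbPieces to a variable of the same name.
; The SaveGameToSlot calls are unreachable, so the function never writes to disk.
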(fn `Sauvegarder`
  (bind _returnvalue (`GameplayStatics.DoesSaveGameExist` (`self.saveName`)))
  (if _returnvalue
    (bind _returnvalue_2 (`GameplayStatics.LoadGameFromSlot` (`self.saveName`)))
    (else
      (bind _returnvalue_3 (`GameplayStatics.CreateSaveGameObject` "BP_Sauvegarde_C"))))
  (set `self.nbPieces` (`self.nbPieces`)))