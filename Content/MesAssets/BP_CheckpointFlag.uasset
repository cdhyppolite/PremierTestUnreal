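; BP_CheckpointFlag is a checkpoint flag that becomes the current one when BP_LavaMan enters its box collider.
; On overlap it clears CurrentFlag on every BP_CheckpointFlag in the level, then sets its own.
; It plays a shake animation, waits its length, then returns to the looping "Before" animation.
; If not yet Actif, it then swaps in a dynamic material with color-variant albedo, normal and roughness textures and marks itself Actif.
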(event `self.BoxCollider.OnComponentBeginOverlap`
  (params (OverlappedComponent :type "PrimitiveComponent Object Reference") (OtherActor :type "Actor Object Reference") (OtherComp :type "PrimitiveComponent Object Reference") (OtherBodyIndex :type Integer) (bFromSweep :type Boolean) (SweepResult :type "HitResult Structure (by ref)"))
  (bind _checkpointflag (`self.CheckpointFlag`))
  (cast `/Game/MesAssets/BP_LavaMan` OtherActor)
  (if (`self.currentFlag`)
    (`KismetSystemLibrary.PrintString` "current"))
  (bind _outactors (`GameplayStatics.GetAllActorsOfClass` "BP_CheckpointFlag_C"))
  (for _array_element _outactors
    (set `/Game/MesAssets/BP_CheckpointFlag.currentFlag` false _array_element))
  (set `self.currentFlag` true)
  ;[1 1 1] Changer Anim
  (`SkeletalMeshComponent.PlayAnimation` _checkpointflag "/Game/MesAssets/Odyssey/CheckpointFlag/Anim/CheckpointFlag_Anim_Armature_Shake.CheckpointFlag_Anim_Armature_Shake" false)
  (`KismetSystemLibrary.Delay` (`self.animLength`))
  (`SkeletalMeshComponent.PlayAnimation` _checkpointflag "/Game/MesAssets/Odyssey/CheckpointFlag/Anim/CheckpointFlag_Anim_Armature_Before.CheckpointFlag_Anim_Armature_Before" true)
  (if (not (`self.actif`))
    (`self.changerCouleurs`)))

(fn `changerCouleurs`
  (bind _checkpointflag (`self.CheckpointFlag`))
  (bind _couleurs (`self.couleurs`))
  (bind _returnvalue (`PrimitiveComponent.CreateDynamicMaterialInstance` _checkpointflag 0 "/Game/MesAssets/Odyssey/CheckpointFlag/Textures/FlagMT.FlagMT" "None"))
  (`MaterialInstanceDynamic.SetTextureParameterValue` _returnvalue "alb_couleur" (`|GetArrayItem` _couleurs))
  (`MaterialInstanceDynamic.SetTextureParameterValue` _returnvalue "nrm_couleur" (`|GetArrayItem` _couleurs 1))
  (`MaterialInstanceDynamic.SetTextureParameterValue` _returnvalue "rgh_couleur" (`|GetArrayItem` _couleurs 2))
  (`PrimitiveComponent.SetMaterial` _checkpointflag 0 _returnvalue)
  (set `self.actif` true))

(fn `UserConstructionScript`)