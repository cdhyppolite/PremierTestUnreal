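; BP_potionFeu is a single-use fire potion pickup that grants BP_LavaMan temporary fire resistance.
; Its box overlap sets a used flag before the cast, so any overlapping actor consumes it.
; For LavaMan, it enables FireResistance, shows a BP_Timer widget fed the duration, then clears resistance after a matching delay.
; Later overlaps only print an already-used message, as the actor is never destroyed.
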(event `self.ReceiveTick`
  (params (DeltaSeconds :type "Float (single-precision)")))

(event `self.BoxCollider.OnComponentBeginOverlap`
  (params (OverlappedComponent :type "PrimitiveComponent Object Reference") (OtherActor :type "Actor Object Reference") (OtherComp :type "PrimitiveComponent Object Reference") (OtherBodyIndex :type Integer) (bFromSweep :type Boolean) (SweepResult :type "HitResult Structure (by ref)"))
  (bind _temps (`self.temps`))
  (if (not (`self.utilisé`))
    (set `self.utilisé` true)
    (bind _asbp_lava_man (cast `/Game/MesAssets/BP_LavaMan` OtherActor))
    (set `/Game/MesAssets/BP_LavaMan.fireResistance` true _asbp_lava_man)
    ;[0 1 0.5545] Apparaitre Timer
    (bind _returnvalue (`|CreateWidget` "/Game/MesAssets/Autres/Potion/BP_Timer.BP_Timer_C" (`GameplayStatics.GetPlayerController` 0)))
    (`UserWidget.AddToViewport` _returnvalue 0)
    (`/Game/MesAssets/Autres/Potion/BP_Timer.tempsDebut` _returnvalue _temps)
    ;[1 0 0.2723] Désactiver la potion
    (`KismetSystemLibrary.Delay` _temps)
    (set `/Game/MesAssets/BP_LavaMan.fireResistance` false _asbp_lava_man)
    (`KismetSystemLibrary.PrintString` "Fire Off")
    (else
      (`KismetSystemLibrary.PrintString` "Potion déjà utilisée" true true (struct :`R` 1.0 :`B` 0.614498 :`A` 1.0)))))

(fn `UserConstructionScript`)