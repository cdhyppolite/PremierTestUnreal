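; BP_Magma is a lava hazard that kills the BP_LavaMan character on contact.
; When BoxCollider begins overlapping a BP_LavaMan without FireResistance, it passes the negated current Vie to GestionVie, removing all health.
; An unconnected branch holds an alternative response that launches the character with a boosted jump, deals fixed damage, then restores the jump height after a delay.
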(event `self.BoxCollider.OnComponentBeginOverlap`
  (params (OverlappedComponent :type "PrimitiveComponent Object Reference") (OtherActor :type "Actor Object Reference") (OtherComp :type "PrimitiveComponent Object Reference") (OtherBodyIndex :type Integer) (bFromSweep :type Boolean) (SweepResult :type "HitResult Structure (by ref)"))
  ;[1 0.3438 0.6684] Collision personnage avec lave
  (bind _asbp_lava_man (cast `/Game/MesAssets/BP_LavaMan` OtherActor))
  (if (not (`/Game/MesAssets/BP_LavaMan.fireResistance` _asbp_lava_man))
    (`/Game/MesAssets/BP_LavaMan.gestionVie` _asbp_lava_man (* (`/Game/MesAssets/BP_LavaMan.vie` _asbp_lava_man) -1))))

(fn `UserConstructionScript`)