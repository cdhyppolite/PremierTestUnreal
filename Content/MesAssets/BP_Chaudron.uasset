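; Cauldron actor where the lava man player deposits collected coins toward a 20-coin victory goal.
; Overlapping its box adds the carried coins to the deposited total in the player's save object, zeroes the carried count and saves to slot.
; A text counter shows the deposited total, refreshed after each deposit and shortly after BeginPlay.
; Reaching 20 opens the victory level.
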(event `self.ReceiveBeginPlay`
  (bind _asbp_lava_man (cast `/Game/MesAssets/BP_LavaMan` (`GameplayStatics.GetPlayerCharacter` 0)))
  (set `self.PersoRef` _asbp_lava_man)
  (`KismetSystemLibrary.Delay` 0.5)
  (`self.TextCompteurPieces`))

(event `self.BoxColliderPieces.OnComponentBeginOverlap`
  (params (OverlappedComponent :type "PrimitiveComponent Object Reference") (OtherActor :type "Actor Object Reference") (OtherComp :type "PrimitiveComponent Object Reference") (OtherBodyIndex :type Integer) (bFromSweep :type Boolean) (SweepResult :type "HitResult Structure (by ref)"))
  ;[1 1 1] Changer valeur compteur
  (bind _asbp_lava_man (cast `/Game/MesAssets/BP_LavaMan` OtherActor))
  (bind _saveref (`/Game/MesAssets/BP_LavaMan.SaveRef` _asbp_lava_man))
  (set `/Game/MesAssets/Autres/BP_Sauvegarde.nbPiecesDeposerSave` (+ (`/Game/MesAssets/Autres/BP_Sauvegarde.nbPiecesDeposerSave` _saveref) (`/Game/MesAssets/Autres/BP_Sauvegarde.nbPiecesSave` _saveref)) _saveref)
  (bind _output_get (set `/Game/MesAssets/Autres/BP_Sauvegarde.nbPiecesSave` 0 _saveref))
  (set `/Game/MesAssets/BP_LavaMan.nbPiecesPerso` _output_get _asbp_lava_man)
  (`GameplayStatics.SaveGameToSlot` _saveref (`/Game/MesAssets/BP_LavaMan.nomSauvegarde` _asbp_lava_man))
  (`self.TextCompteurPieces`))

(event `TextCompteurPieces`
  (bind _nbpiecesdeposersave (`/Game/MesAssets/Autres/BP_Sauvegarde.nbPiecesDeposerSave` (`/Game/MesAssets/BP_LavaMan.SaveRef` (`self.PersoRef`))))
  ;[1 1 1] Afficher compteur
  (`TextRenderComponent.K2_SetText` (`self.Compteur`) (`|FormatText` "{nbPieces}/20" _nbpiecesdeposersave))
  (if (>= _nbpiecesdeposersave 20)
    (`GameplayStatics.OpenLevelBySoftObjectPtr` "/Game/MesAssets/Niveau/LV_Victoire.LV_Victoire")))

(fn `UserConstructionScript`)