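; BP_SkyBox is a skybox actor that textures a cube mesh to form the surrounding sky.
; On BeginPlay, it creates a dynamic instance of the LavaSkySide material for each of the cube's six material slots.
; Each instance receives its own face texture (top, bottom, front, back, right, left) through a shared texture parameter name, so the faces appear only at runtime, with an empty construction script.
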(event `self.ReceiveBeginPlay`
  (bind _skyboxcube (`self.SkyBoxCube`))
  ;[1 1 1] Haut
  (bind _returnvalue (`PrimitiveComponent.CreateDynamicMaterialInstance` _skyboxcube 1 "/Game/MesAssets/SkyBox/LavaSkySide.LavaSkySide" "None"))
  (`MaterialInstanceDynamic.SetTextureParameterValue` _returnvalue (`self.constNomParam`) (`self.Haut`))
  ;[1 1 1] Bas
  (bind _returnvalue_2 (`PrimitiveComponent.CreateDynamicMaterialInstance` _skyboxcube 3 "/Game/MesAssets/SkyBox/LavaSkySide.LavaSkySide" "None"))
  (`MaterialInstanceDynamic.SetTextureParameterValue` _returnvalue_2 (`self.constNomParam`) (`self.Bas`))
  ;[1 1 1] Avant
  (bind _returnvalue_3 (`PrimitiveComponent.CreateDynamicMaterialInstance` _skyboxcube 0 "/Game/MesAssets/SkyBox/LavaSkySide.LavaSkySide" "None"))
  (`MaterialInstanceDynamic.SetTextureParameterValue` _returnvalue_3 (`self.constNomParam`) (`self.Front`))
  ;[1 1 1] Arrière
  (bind _returnvalue_4 (`PrimitiveComponent.CreateDynamicMaterialInstance` _skyboxcube 2 "/Game/MesAssets/SkyBox/LavaSkySide.LavaSkySide" "None"))
  (`MaterialInstanceDynamic.SetTextureParameterValue` _returnvalue_4 (`self.constNomParam`) (`self.Back`))
  ;[1 1 1] Droite
  (bind _returnvalue_5 (`PrimitiveComponent.CreateDynamicMaterialInstance` _skyboxcube 4 "/Game/MesAssets/SkyBox/LavaSkySide.LavaSkySide" "None"))
  (`MaterialInstanceDynamic.SetTextureParameterValue` _returnvalue_5 (`self.constNomParam`) (`self.Right`))
  ;[1 1 1] Gauche
  (bind _returnvalue_6 (`PrimitiveComponent.CreateDynamicMaterialInstance` _skyboxcube 5 "/Game/MesAssets/SkyBox/LavaSkySide.LavaSkySide" "None"))
  (`MaterialInstanceDynamic.SetTextureParameterValue` _returnvalue_6 (`self.constNomParam`) (`self.Left`)))

(fn `UserConstructionScript`)