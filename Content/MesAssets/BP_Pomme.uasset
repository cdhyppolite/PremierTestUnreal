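; BP_Pomme is an apple actor that damages BP_LavaMan on overlap and starts simulating physics when hit.
; On BeginPlay it creates a dynamic material with a randomly picked color texture.
; Sphere collider overlap passes size-based damage to the character's GestionVie, multiplying Degat by the actor's scale vector length.
; A hit on the same collider enables physics on the apple mesh and prints a debug message.
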(event `self.ReceiveBeginPlay`
  (`self.couleursRandom`))

(event `couleursRandom`
  (bind _pomme (`self.Pomme`))
  ;[1 0.7537 0] Couleur random
  (bind _returnvalue (`PrimitiveComponent.CreateDynamicMaterialInstance` _pomme 0 "/Game/MesAssets/Odyssey/Pomme/PommeMT.PommeMT" "None"))
  (`MaterialInstanceDynamic.SetTextureParameterValue` _returnvalue "couleur" (`KismetArrayLibrary.Array_Random` (`self.couleurs`)))
  (`PrimitiveComponent.SetMaterial` _pomme 0 _returnvalue))

(event `self.SphereCollider.OnComponentBeginOverlap`
  (params (OverlappedComponent :type "PrimitiveComponent Object Reference") (OtherActor :type "Actor Object Reference") (OtherComp :type "PrimitiveComponent Object Reference") (OtherBodyIndex :type Integer) (bFromSweep :type Boolean) (SweepResult :type "HitResult Structure (by ref)"))
  (bind _asbp_lava_man (cast `/Game/MesAssets/BP_LavaMan` OtherActor))
  (`/Game/MesAssets/BP_LavaMan.gestionVie` _asbp_lava_man (`KismetMathLibrary.FTrunc` (* (`self.degat`) (`KismetMathLibrary.VSize` (`self.GetActorScale3D`))))))

(event `self.SphereCollider.OnComponentHit`
  (params (HitComponent :type "PrimitiveComponent Object Reference") (OtherActor :type "Actor Object Reference") (OtherComp :type "PrimitiveComponent Object Reference") (NormalImpulse :type "Vector Structure") (Hit :type "HitResult Structure (by ref)"))
  (`PrimitiveComponent.SetSimulatePhysics` (`self.Pomme`) true)
  (`KismetSystemLibrary.PrintText` "hit"))

(fn `UserConstructionScript`)