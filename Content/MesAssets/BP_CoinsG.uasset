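; BP_CoinsG is a collectible coin for the BP_LavaMan character.
; On BeginPlay, if CouleurRandom is set, a dynamic material instance gives its skeletal mesh a random color.
; When BP_LavaMan overlaps the sphere collider, the coin calls its GestionVie function and increments the saved coin count.
; It writes the save slot immediately, syncs the character's counter from the save, then destroys itself.
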(event `self.ReceiveBeginPlay`
  (if (`self.couleurRandom`)
    (bind _returnvalue (`PrimitiveComponent.CreateDynamicMaterialInstance` (`self.SkeletalMesh`) 0 null "None"))
    (`MaterialInstanceDynamic.SetVectorParameterValue` _returnvalue "Couleur" (`KismetMathLibrary.MakeColor` (`KismetMathLibrary.RandomFloatInRange` 0.0 1.0) (`KismetMathLibrary.RandomFloatInRange` 0.0 1.0) (`KismetMathLibrary.RandomFloatInRange` 0.0 1.0)))))

(event `self.SphereCollider.OnComponentBeginOverlap`
  (params (OverlappedComponent :type "PrimitiveComponent Object Reference") (OtherActor :type "Actor Object Reference") (OtherComp :type "PrimitiveComponent Object Reference") (OtherBodyIndex :type Integer) (bFromSweep :type Boolean) (SweepResult :type "HitResult Structure (by ref)"))
  (bind _asbp_lava_man (cast `/Game/MesAssets/BP_LavaMan` OtherActor))
  (`/Game/MesAssets/BP_LavaMan.gestionVie` _asbp_lava_man 5)
  (bind _saveref (`/Game/MesAssets/BP_LavaMan.SaveRef` _asbp_lava_man))
  (bind _output_get (set `/Game/MesAssets/Autres/BP_Sauvegarde.nbPiecesSave` (+ 1 (`/Game/MesAssets/Autres/BP_Sauvegarde.nbPiecesSave` _saveref)) _saveref))
  (`GameplayStatics.SaveGameToSlot` _saveref (`/Game/MesAssets/BP_LavaMan.nomSauvegarde` _asbp_lava_man))
  (set `/Game/MesAssets/BP_LavaMan.nbPiecesPerso` _output_get _asbp_lava_man)
  (`self.K2_DestroyActor`))

(fn `UserConstructionScript`)